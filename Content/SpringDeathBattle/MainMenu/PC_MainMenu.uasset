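; Main menu player controller that swaps menu screens and hosts multiplayer sessions.
; WidgetSwap replaces the active widget with the main menu, server list, customization or credits screen by index, and a looping timer recreates it if invalid.
; A second timer keeps reloading player name and character from the setup save.
; Hosting creates a session, optionally LAN, then opens Platform as a listen server, and EndPlay restores game-only input.
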(event `self.ReceiveBeginPlay`
  (set `self.bShowMouseCursor` true)
  (`KismetSystemLibrary.Delay` 2.0)
  (`KismetSystemLibrary.K2_SetTimerDelegate` (delegate `CheckForWidget`) 0.5 true)
  (`KismetSystemLibrary.K2_SetTimerDelegate` (delegate `gfdsafdzsgds`) 1.0 true))

(event `gfdsafdzsgds`
  (bind _returnvalue (`GameplayStatics.DoesSaveGameExist` "PlayerSetupSave"))
  (if _returnvalue
    (bind _returnvalue_2 (`GameplayStatics.LoadGameFromSlot` "PlayerSetupSave"))
    (bind _assave_spring_death_battle (cast `/Game/SpringDeathBattle/Blueprints/Base/Save_SpringDeathBattle` _returnvalue_2))
    (bind (_playername _playercharacter) (break `/Game/SpringDeathBattle/Blueprints/Base/PlayerInfo` (`/Game/SpringDeathBattle/Blueprints/Base/Save_SpringDeathBattle.S_PlayerInfo` _assave_spring_death_battle)))
    (set `self.PlayerName` _playername)
    (set `self.PlayerChar` _playercharacter)))

(event `CheckForWidget`
  (`/Engine/EditorBlueprintResources/StandardMacros.IsValid` (`self.ActiveWidget`)
    (:`Is Not Valid`
      (`self.WidgetSwap`))))

(event `PlayerHostGame`
  (set `self.bShowMouseCursor` false)
  (`CreateSessionCallbackProxy.CreateSession` self 8 (`self.LAN?`)
    (:`OnSuccess`
      (`GameplayStatics.OpenLevel` "Platform" true "listen"))
    (:`OnFailure`
      (set `self.bShowMouseCursor` true)
      (`KismetSystemLibrary.PrintString` "Hosting game failed!" true true (struct :`R` 0.51 :`B` 0.023174 :`A` 1.0) 99.0))))

(event `self.ReceiveEndPlay`
  (params (EndPlayReason :type "EEndPlayReason Enum" :default "Destroyed"))
  (bind _ref_mainmenuwidg (`self.Ref_MainMenuWidg`))
  (`WidgetBlueprintLibrary.SetFocusToGameViewport`)
  (`WidgetBlueprintLibrary.SetInputMode_GameOnly` self)
  (set `self.bShowMouseCursor` false)
  (`/Engine/EditorBlueprintResources/StandardMacros.IsValid` _ref_mainmenuwidg
    (:`Is Valid`
      (`Widget.RemoveFromParent` _ref_mainmenuwidg))))

(event `WidgetSwap`
  (`/Engine/EditorBlueprintResources/StandardMacros.IsValid` (`self.ActiveWidget`)
    (:`Is Valid`
      (`Widget.RemoveFromParent` (`self.ActiveWidget`)))
    (:`Is Not Valid`
      _))
  (switch `int` (`self.WidgetArray`)
    (:`0`
      (bind _returnvalue (`|CreateWidget` "/Game/SpringDeathBattle/MainMenu/Widgets/Widg_MainMenu.Widg_MainMenu_C"))
      (bind _output_get (set `self.ActiveWidget` _returnvalue))
      (`UserWidget.AddToViewport` _output_get 0))
    (:`1`
      (bind _returnvalue_2 (`|CreateWidget` "/Game/SpringDeathBattle/MainMenu/Widgets/Widg_JoinServerList.Widg_JoinServerList_C"))
      (bind _output_get_2 (set `self.ActiveWidget` _returnvalue_2))
      (`UserWidget.AddToViewport` _output_get_2 0))
    (:`2`
      (bind _returnvalue_3 (`|CreateWidget` "/Game/SpringDeathBattle/MainMenu/Widgets/Customization.Customization_C"))
      (bind _output_get_3 (set `self.ActiveWidget` _returnvalue_3))
      (`UserWidget.AddToViewport` _output_get_3 0))
    (:`3`
      (bind _returnvalue_4 (`|CreateWidget` "/Game/SpringDeathBattle/MainMenu/Widgets/Widg_Credits.Widg_Credits_C"))
      (bind _output_get_4 (set `self.ActiveWidget` _returnvalue_4))
      (`UserWidget.AddToViewport` _output_get_4 0))))

(fn `UserConstructionScript`)
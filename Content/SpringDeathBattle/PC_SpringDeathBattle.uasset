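; Player controller for Spring Death Battle, handling a player's match UI, ready-up, round timer and session exit.
; BeginPlay loads saved player info, creates HUD and scoreboard, and starts polling for the ready prompt with player counts.
; Delay loops poll flags to start the countdown and show the scoreboard at round over.
; Tick possesses a spawned spectator when pawnless; Escape returns to the main menu, destroying the session first on authority.
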(event `check server ready?`
  (bind _ref_widgetready (`self.Ref-WidgetReady`))
  (if (`self.ServerWaitingForRoundToStart?`)
    (`/Engine/EditorBlueprintResources/StandardMacros.IsValid` (`self.Ref-WidgetReady`)
      (:`Is Valid`
        _)
      (:`Is Not Valid`
        (bind _returnvalue (`|CreateWidget` "/Game/SpringDeathBattle/Blueprints/Widgets/Widget-Ready.Widget-Ready_C" self))
        (set `self.Ref-WidgetReady` _returnvalue)
        (`UserWidget.AddToViewport` _returnvalue 0)))
    (bind _aswidget__ready (cast `/Game/SpringDeathBattle/Blueprints/Widgets/Widget-Ready` (`self.Ref-WidgetReady`)))
    (`TextBlock.SetText` (`/Game/SpringDeathBattle/Blueprints/Widgets/Widget-Ready.TextBlock_AmountOfReadyPlayers` _aswidget__ready) (`KismetTextLibrary.Conv_IntToText` (`self.PlayersReady`)))
    (`TextBlock.SetText` (`/Game/SpringDeathBattle/Blueprints/Widgets/Widget-Ready.TextBlock_AmountOfNeededReadyPlayers` _aswidget__ready) (`KismetTextLibrary.Conv_IntToText` (`self.PlayersNeededReady`)))
    (else
      (`/Engine/EditorBlueprintResources/StandardMacros.IsValid` _ref_widgetready
        (:`Is Valid`
          (`Widget.RemoveFromParent` _ref_widgetready)
          (set `self.Ref-WidgetReady` null))))))

(event `self.ReceiveBeginPlay`
  (`self.SaveGameCheck`)
  (`/Engine/EditorBlueprintResources/StandardMacros.IsValid` (`self.Ref-WidgetScoreboard`)
    (:`Is Valid`
      _)
    (:`Is Not Valid`
      (bind _returnvalue (`|CreateWidget` "/Game/SpringDeathBattle/Blueprints/Widgets/Widget_Scoreboard.Widget_Scoreboard_C"))
      (bind _output_get (set `self.Ref-WidgetScoreboard` _returnvalue))
      (`UserWidget.AddToViewport` _output_get 0)
      (`Widget.SetVisibility` _output_get "Hidden")))
  (bind _returnvalue_2 (`|CreateWidget` "/Game/SpringDeathBattle/Blueprints/Widgets/Widget-HUD.Widget-HUD_C" self))
  (`/Engine/EditorBlueprintResources/StandardMacros.IsValid` _returnvalue_2
    (:`Is Valid`
      (`UserWidget.AddToViewport` _returnvalue_2 0)
      (`KismetSystemLibrary.K2_SetTimerDelegate` (delegate `check server ready?`) 0.5 true)
      (if (`self.ActivateTimer?`) :!label _label
        (bind _returnvalue_3 (`KismetSystemLibrary.K2_SetTimerDelegate` (delegate `ReduceTimer`) 0.25 true))
        (else
          (`KismetSystemLibrary.Delay` 0.2 :!label _label_2)
          (goto _label))))))

(event `ReduceTimer`
  (bind _ref_widgetscoreboard (`self.Ref-WidgetScoreboard`))
  (bind _output_get (set `self.RoundTimeLeft` (- (`self.RoundTimeLeft`) 0.25)))
  (if (<= _output_get 0.0)
    (if (`self.RoundOver`) :!label _label_3
      (set `self.ActivateTimer?` false)
      (`KismetSystemLibrary.K2_ClearAndInvalidateTimerHandle` (stale `self.ReceiveBeginPlay` _returnvalue_3))
      (`Widget.SetVisibility` _ref_widgetscoreboard "Visible")
      (`KismetSystemLibrary.Delay` 0.2)
      (goto _label_3)
      (else
        (`Widget.SetVisibility` _ref_widgetscoreboard "Hidden")
        (goto _label_2)))))

(event `InputAction|Ready`
  (params (Key :type "Key Structure"))
  (:`Pressed`
    (`/Engine/EditorBlueprintResources/StandardMacros.DoOnce` false :!label _label_4
      (:`Completed`
        (`self.ReadyCheck`))))
  (:`Released`
    (goto _label_4 :!via `Reset`)))

(event `ReadyCheck`
  (set `self.ReadyForMatch?` (not (`self.ReadyForMatch?`))))

(event `self.ReceiveTick`
  (params (DeltaSeconds :type "Float (single-precision)"))
  (`/Engine/EditorBlueprintResources/StandardMacros.IsValid` (`self.K2_GetPawn`)
    (:`Is Not Valid`
      (bind _returnvalue (`|SpawnActorFromClass` "/Game/SpringDeathBattle/Blueprints/DSB_Spectator.DSB_Spectator_C" (`KismetMathLibrary.MakeTransform` (0.0 0.0 500.0)) "AdjustIfPossibleButAlwaysSpawn" "OverrideRootScale" null null))
      (`self.Possess` _returnvalue))))

(event `Key|Escape`
  (params (Key :type "Key Structure"))
  (:`Pressed`
    (`/Engine/EditorBlueprintResources/ActorMacros.Switch Has Authority`
      (:`Authority`
        (`DestroySessionCallbackProxy.DestroySession` self
          (:`OnSuccess`
            _)))
      (:`Remote`
        _))
    (`GameplayStatics.OpenLevel` "MainMenu")))

(event `Key|Tab`
  (params (Key :type "Key Structure"))
  (:`Pressed`
    (if (not (`self.RoundOver`))
      (`/Engine/EditorBlueprintResources/StandardMacros.IsValid` (`self.Ref-WidgetScoreboard`)
        (:`Is Valid`
          (`Widget.SetVisibility` (`self.Ref-WidgetScoreboard`) "Visible"))
        (:`Is Not Valid`
          (bind _returnvalue (`|CreateWidget` "/Game/SpringDeathBattle/Blueprints/Widgets/Widget_Scoreboard.Widget_Scoreboard_C" self))
          (bind _output_get (set `self.Ref-WidgetScoreboard` _returnvalue))
          (`UserWidget.AddToViewport` _output_get 0)))))
  (:`Released`
    (if (not (`self.RoundOver`))
      (`Widget.SetVisibility` (`self.Ref-WidgetScoreboard`) "Hidden"))))

(fn `LoadGame`
  (bind _returnvalue (`GameplayStatics.LoadGameFromSlot` (`self.PlayerSetupSave`)))
  (bind _assave_spring_death_battle (cast `/Game/SpringDeathBattle/Blueprints/Base/Save_SpringDeathBattle` _returnvalue))
  (bind (_playername _playercharacter) (break `/Game/SpringDeathBattle/Blueprints/Base/PlayerInfo` (`/Game/SpringDeathBattle/Blueprints/Base/Save_SpringDeathBattle.S_PlayerInfo` _assave_spring_death_battle)))
  (setmembers `/Game/SpringDeathBattle/Blueprints/Base/PlayerInfo` :`StructRef` (`self.PlayerInfo`) :`PlayerName` _playername :`PlayerCharacter` _playercharacter)
  (set `self.PlayerName` _playername)
  (set `self.PlayerCharacter` _playercharacter))

(fn `OnRep_Ref_PState`)

(fn `SaveGame`
  (`/Engine/EditorBlueprintResources/StandardMacros.IsValid` (`self.Ref_PlayerSaveGame`)
    (:`Is Not Valid`
      (bind _returnvalue (`GameplayStatics.CreateSaveGameObject` "/Game/SpringDeathBattle/Blueprints/Base/Save_SpringDeathBattle.Save_SpringDeathBattle_C"))
      (bind _output_get (set `self.Ref_PlayerSaveGame` _returnvalue))
      (set `/Game/SpringDeathBattle/Blueprints/Base/Save_SpringDeathBattle.S_PlayerInfo` (`self.PlayerInfo`) _output_get))))

(fn `SaveGameCheck`
  (bind _returnvalue (`GameplayStatics.DoesSaveGameExist` (`self.PlayerSetupSave`)))
  (if _returnvalue
    (`self.LoadGame`)
    (`self.SaveGame`)
    (else
      (`self.SaveGame`))))

(fn `UserConstructionScript`)
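; Pickup actor that grants a power-up to a SpringBattleBase actor that overlaps its sphere, then destroys itself.
; A RandomizeType event picks the pickup's type at random from the SpawningPowerUps array; nothing in this Blueprint calls it.
; On overlap, a switch on the type applies the effect, with Double Jump the only case wired, and the pickup is destroyed whatever its type.
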(event `RandomizeType`
  (bind _spawningpowerups (`self.SpawningPowerUps`))
  (set `self.PowerUpType` (`|GetArrayItem` _spawningpowerups (`KismetMathLibrary.RandomIntegerInRange` 0 (- (`KismetArrayLibrary.Array_Length` _spawningpowerups) 1)))))

(event `self.Sphere.OnComponentBeginOverlap`
  (params (OverlappedComponent :type "PrimitiveComponent Object Reference") (OtherActor :type "Actor Object Reference") (OtherComp :type "PrimitiveComponent Object Reference") (OtherBodyIndex :type Integer) (bFromSweep :type Boolean) (SweepResult :type "HitResult Structure (by ref)"))
  (bind _asspring_battle_base (cast `/Game/SpringDeathBattle/Blueprints/SpringBattleBase` OtherActor))
  (`|ExecutionSequence`
    (:`then_0`
      (switch `/Game/SpringDeathBattle/Blueprints/PowerUp/Enum_PowerUp` (`self.PowerUpType`)
        (:`NewEnumerator0`
          (`/Game/SpringDeathBattle/Blueprints/SpringBattleBase.PowerUp - Double Jump` _asspring_battle_base)
          (`self.K2_DestroyActor`))))
    (:`then_1`
      (`self.K2_DestroyActor`))))

(fn `UserConstructionScript`)
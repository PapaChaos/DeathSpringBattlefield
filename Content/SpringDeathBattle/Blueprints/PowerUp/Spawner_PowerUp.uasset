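; Power-up spawner for the SpringDeathBattle mode that keeps a pickup respawning above its mesh.
; On authority BeginPlay it caches the game mode, gathers the enabled types from the ViablePowerUps map if randomizing, and can spawn immediately.
; Each spawned PowerUp gets either a random type from that list or a fixed CertainPowerUp.
; Server Tick runs the respawn timer once the match starts, resetting it while a pickup exists.
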(event `self.ReceiveBeginPlay`
  (`/Engine/EditorBlueprintResources/ActorMacros.Switch Has Authority`
    (:`Authority`
      (bind _asgm_spring_death_battle (cast `/Game/SpringDeathBattle/GM_SpringDeathBattle` (`GameplayStatics.GetGameMode`)))
      (set `self.Ref_GM` _asgm_spring_death_battle)
      (if (`self.Randomize PowerUp?`)
        (bind _values (`BlueprintMapLibrary.Map_Values` (`self.ViablePowerUps`)))
        (for (_array_element _array_index) _values
          (if _array_element
            (bind _keys (`BlueprintMapLibrary.Map_Keys` (`self.ViablePowerUps`)))
            (`KismetArrayLibrary.Array_Add` (`self.SpawningPowerUps`) (`|GetArrayItem` _keys _array_index)))))
      (if (`self.StartSpawned?`)
        (`self.Spawn PowerUp`)))))

(event `Spawn PowerUp`
  (bind _returnvalue (`KismetMathLibrary.MakeTransform` (+ (.location (`SceneComponent.K2_GetComponentToWorld` (`self.StaticMeshComponent`))) (0.0 0.0 100.0)) (.rotation (`SceneComponent.K2_GetComponentToWorld` (`self.StaticMeshComponent`)))))
  (if (`self.Randomize PowerUp?`) :!label _label
    (bind _returnvalue_2 (`|SpawnActorFromClass` "/Game/SpringDeathBattle/Blueprints/PowerUp/PowerUp.PowerUp_C" _returnvalue "AlwaysSpawn" "OverrideRootScale" null null))
    (set `/Game/SpringDeathBattle/Blueprints/PowerUp/PowerUp.SpawningPowerUps` (`self.SpawningPowerUps`) _returnvalue_2)
    (`/Game/SpringDeathBattle/Blueprints/PowerUp/PowerUp.RandomizeType` _returnvalue_2)
    (`/Engine/EditorBlueprintResources/StandardMacros.IsValid` _returnvalue_2
      (:`Is Valid`
        (set `self.SpawnedPowerUp` _returnvalue_2)))
    (else
      (bind _returnvalue_3 (`|SpawnActorFromClass` "/Game/SpringDeathBattle/Blueprints/PowerUp/PowerUp.PowerUp_C" _returnvalue "AlwaysSpawn" "OverrideRootScale" null null))
      (set `/Game/SpringDeathBattle/Blueprints/PowerUp/PowerUp.PowerUpType` (`self.CertainPowerUp`) _returnvalue_3)
      (`/Engine/EditorBlueprintResources/StandardMacros.IsValid` _returnvalue_3
        (:`Is Valid`
          (set `self.SpawnedPowerUp` _returnvalue_3))))))

(event `self.ReceiveTick`
  (params (DeltaSeconds :type "Float (single-precision)"))
  (`/Engine/EditorBlueprintResources/ActorMacros.Switch Has Authority`
    (:`Authority`
      (if (`/Game/SpringDeathBattle/GM_SpringDeathBattle.MatchStart` (`self.Ref_GM`))
        (`/Engine/EditorBlueprintResources/StandardMacros.IsValid` (`self.SpawnedPowerUp`)
          (:`Is Valid`
            (set `self.Timer` 0.0))
          (:`Is Not Valid`
            (bind _output_get (set `self.Timer` (+ DeltaSeconds (`self.Timer`))))
            (if (>= _output_get (`self.SpawnTime`))
              (goto _label))))))))

(fn `UserConstructionScript`)
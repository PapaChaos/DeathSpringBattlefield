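; Game mode for Spring Death Battle that runs timed multiplayer kill-count rounds from ready-up to winner announcement.
; It tracks joined player controllers with parallel kill and death arrays, starting a round once a majority is ready.
; During rounds, looping timers respawn players at random PlayerStarts and push scoreboards to each controller.
; At round end it destroys pawns, announces the top killer, then returns to waiting after a short delay.
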(event `ClearLastRound`
  (`/Engine/EditorBlueprintResources/StandardMacros.DoOnce` false :!label _label
    (:`Completed`
      (for _array_element (`self.PlayersThisMatch`)
        (set `/Game/SpringDeathBattle/PC_SpringDeathBattle.ReadyForMatch?` false _array_element)
        (set `/Game/SpringDeathBattle/PC_SpringDeathBattle.RoundOver` false _array_element))
      (for _array_element_2 (`self.PlayersThisMatch`)
        (set `/Game/SpringDeathBattle/PC_SpringDeathBattle.ServerWaitingForRoundToStart?` true _array_element_2))
      (`self.Loop`)
      (goto _label :!via `Reset`))))

(event `CheckPlayerStarts`
  (bind _playerstart (`self.PlayerStart`))
  (for (_array_element _array_index) _playerstart
    (`/Engine/EditorBlueprintResources/StandardMacros.IsValid` _array_element
      (:`Is Not Valid`
        (`KismetArrayLibrary.Array_Remove` _playerstart _array_index)))))

(event `self.ReceiveBeginPlay`
  (bind _outactors (`GameplayStatics.GetAllActorsOfClass` "/Script/Engine.PlayerStart"))
  (set `self.PlayerStart` _outactors)
  (`self.Loop`)
  (bind _asgsb_spring_death_battle (cast `/Game/SpringDeathBattle/Blueprints/Base/GSB_SpringDeathBattle` (`GameplayStatics.GetGameState`) :!label _label_2)
    (:`then`
      (bind _output_get (set `self.Ref_SpringDeathBattle` _asgsb_spring_death_battle))
      (`/Engine/EditorBlueprintResources/StandardMacros.IsValid` _output_get
        (:`Is Not Valid`
          _)))
    (:`CastFailed`
      (`KismetSystemLibrary.PrintString` "Loop error GSB")))
  (`KismetSystemLibrary.Delay` 0.2)
  (goto _label_2))

(event `CheckReadyToStart`
  (bind _playersthismatch (`self.PlayersThisMatch`))
  (bind _playerkills (`self.PlayerKills`))
  (bind _playerdeaths (`self.PlayerDeaths`))
  (bind _returnvalue (`KismetArrayLibrary.Array_Length` (`self.PlayersThisMatch`)))
  (if (> (`KismetArrayLibrary.Array_Length` (`self.PlayersThisMatch`)) 0)
    (set `self.AmountOfPlayersReady` 0)
    (`KismetArrayLibrary.Array_Clear` (`self.ServerAllPlayerNames`))
    (bind _output_get (set `self.AmountOfPlayersReadyNeeded` (+ (/ (`KismetArrayLibrary.Array_Length` _playersthismatch) 2) 1)))
    (for _array_element _playersthismatch
      (set `/Game/SpringDeathBattle/PC_SpringDeathBattle.ServerWaitingForRoundToStart?` true _array_element)
      (if (`/Game/SpringDeathBattle/PC_SpringDeathBattle.ReadyForMatch?` _array_element)
        (set `self.AmountOfPlayersReady` (+ (`self.AmountOfPlayersReady`) 1))))
    (for _array_element_2 (`self.PlayersThisMatch`)
      (set `/Game/SpringDeathBattle/PC_SpringDeathBattle.PlayersReady` (`self.AmountOfPlayersReady`) _array_element_2)
      (set `/Game/SpringDeathBattle/PC_SpringDeathBattle.PlayersNeededReady` _output_get _array_element_2)
      (`KismetArrayLibrary.Array_Add` (`/Game/SpringDeathBattle/PC_SpringDeathBattle.AllPlayersNames` _array_element_2)))
    (`self.ScoreboardUpdate`)
    (if (>= (`self.AmountOfPlayersReady`) _output_get)
      (`KismetArrayLibrary.Array_Resize` (`self.PlayerKills`) _returnvalue)
      (`KismetArrayLibrary.Array_Resize` (`self.PlayerDeaths`) _returnvalue)
      (for (_ _array_index) _playerkills
        (`KismetArrayLibrary.Array_Set` _playerkills _array_index))
      (for (_ _array_index_2) _playerdeaths
        (`KismetArrayLibrary.Array_Set` _playerdeaths _array_index_2))
      (for _array_element_3 (`self.PlayersThisMatch`)
        (set `/Game/SpringDeathBattle/PC_SpringDeathBattle.ServerWaitingForRoundToStart?` false _array_element_3)
        (set `/Game/SpringDeathBattle/PC_SpringDeathBattle.RoundTimeLeft` (`self.RoundLength`) _array_element_3)
        (set `/Game/SpringDeathBattle/PC_SpringDeathBattle.ActivateTimer?` true _array_element_3))
      (`self.StartRound`))))

(event `Loop`
  (`self.CheckReadyToStart` :!label _label_3)
  (if (`self.MatchStart`)
    (bind _returnvalue (`KismetSystemLibrary.K2_SetTimerDelegate` (delegate `Server Spawn`) 1.0 true))
    (else
      (`KismetSystemLibrary.Delay` 1.0)
      (goto _label_3))))

(event `SpawnTimerStop`
  (`KismetSystemLibrary.K2_ClearAndInvalidateTimerHandle` (stale `Loop` _returnvalue)))

(event `ScoreboardUpdate`
  (`KismetArrayLibrary.Array_Clear` (`self.ServerAllPlayerNames`))
  (for _array_element (`self.PlayersThisMatch`)
    (`KismetArrayLibrary.Array_Add` (`self.ServerAllPlayerNames`) (`/Game/SpringDeathBattle/PC_SpringDeathBattle.PlayerName` _array_element)))
  (for _array_element_2 (`self.PlayersThisMatch`)
    (set `/Game/SpringDeathBattle/PC_SpringDeathBattle.AllPlayersNames` (`self.ServerAllPlayerNames`) _array_element_2)
    (set `/Game/SpringDeathBattle/PC_SpringDeathBattle.AllPlayersKills` (`self.PlayerKills`) _array_element_2)))

(event `SBUIG`
  (`self.ScoreboardUpdate`))

(event `Server Spawn`
  (bind _playerstart (`self.PlayerStart`))
  (bind _ref_pc (`self.Ref-PC`))
  (bind _returnvalue (`Controller.K2_GetPawn` (`self.Ref-PC`)))
  (`self.CheckPlayerStarts`)
  (for (_array_element _array_index) (`self.PlayersThisMatch`)
    (bind _output_get (set `self.Ref-PC` _array_element))
    (`/Engine/EditorBlueprintResources/StandardMacros.IsValid` _output_get
      (:`Is Valid`
        (`/Engine/EditorBlueprintResources/StandardMacros.IsValid` _returnvalue
          (:`Is Valid`
            (if (== _returnvalue "/Game/SpringDeathBattle/Spec_SprintDeathBattle.Spec_SprintDeathBattle")
              (`self.CreateCharForPlayer` (`/Game/SpringDeathBattle/PC_SpringDeathBattle.PlayerCharacter` _ref_pc) (`|GetArrayItem` _playerstart (`KismetMathLibrary.RandomIntegerInRange` 0 (- (`KismetArrayLibrary.Array_Length` _playerstart) 1))) _ref_pc (`/Game/SpringDeathBattle/PC_SpringDeathBattle.PlayerName` _ref_pc) :!label _label_4)))
          (:`Is Not Valid`
            (goto _label_4))))
      (:`Is Not Valid`
        (`KismetArrayLibrary.Array_Remove` (`self.PlayersThisMatch`) _array_index)))))

(event `StartRound`
  (set `self.MatchStart` true)
  (bind _returnvalue (`KismetSystemLibrary.K2_SetTimerDelegate` (delegate `SBUIG`) 0.5 true))
  (`KismetSystemLibrary.K2_SetTimerDelegate` (delegate `EndRound`) (`self.RoundLength`)))

(event `EndRound`
  (bind _playersthismatch (`self.PlayersThisMatch`))
  (bind (_indexofmaxvalue _maxvalue) (`KismetMathLibrary.MaxOfIntArray` (`self.PlayerKills`)))
  (set `self.MatchStart` false)
  (`self.SpawnTimerStop`)
  (`KismetSystemLibrary.K2_ClearAndInvalidateTimerHandle` (stale `StartRound` _returnvalue))
  (for _array_element _playersthismatch
    (`self.K2_DestroyActor` (`Controller.K2_GetPawn` _array_element))
    (set `/Game/SpringDeathBattle/PC_SpringDeathBattle.WinnerName` (`/Game/SpringDeathBattle/PC_SpringDeathBattle.PlayerName` (`|GetArrayItem` _playersthismatch _indexofmaxvalue)) _array_element)
    (set `/Game/SpringDeathBattle/PC_SpringDeathBattle.WinnerKills` _maxvalue _array_element)
    (set `/Game/SpringDeathBattle/PC_SpringDeathBattle.RoundOver` true _array_element))
  (`KismetSystemLibrary.Delay` 5.0)
  (`self.ClearLastRound`))

(event `self.K2_PostLogin`
  (params (NewPlayer :type "PlayerController Object Reference"))
  ;[1 1 1] OnPostLogin
  (bind _aspc_spring_death_battle (cast `/Game/SpringDeathBattle/PC_SpringDeathBattle` NewPlayer :!label _label_5)
    (:`then`
      (`/Engine/EditorBlueprintResources/ActorMacros.Switch Has Authority`
        (:`Authority`
          (bind _returnvalue (`KismetArrayLibrary.Array_Add` (`self.PlayersThisMatch`) _aspc_spring_death_battle))
          (`KismetArrayLibrary.Array_Insert` (`self.PlayerKills`) 0 _returnvalue)
          (`KismetArrayLibrary.Array_Insert` (`self.PlayerDeaths`) 0 _returnvalue)
          (`KismetSystemLibrary.PrintString` (`KismetStringLibrary.Concat_StrStr` (`KismetTextLibrary.Conv_TextToString` (`/Game/SpringDeathBattle/PC_SpringDeathBattle.PlayerName` _aspc_spring_death_battle)) " has joined the server.")))))
    (:`CastFailed`
      (`KismetSystemLibrary.Delay` 0.2)
      (goto _label_5))))

(event `self.K2_OnLogout`
  (params (ExitingController :type "Controller Object Reference"))
  (bind _playersthismatch (`self.PlayersThisMatch`))
  ;[1 1 1] OnLogout
  (bind _aspc_spring_death_battle (cast `/Game/SpringDeathBattle/PC_SpringDeathBattle` ExitingController :!label _label_6)
    (:`then`
      (`/Engine/EditorBlueprintResources/ActorMacros.Switch Has Authority`
        (:`Authority`
          (bind _returnvalue (`KismetArrayLibrary.Array_Find` _playersthismatch _aspc_spring_death_battle))
          (`KismetArrayLibrary.Array_Remove` (`self.PlayerKills`) _returnvalue)
          (`KismetArrayLibrary.Array_Remove` (`self.PlayerDeaths`) _returnvalue)
          (`KismetArrayLibrary.Array_RemoveItem` _playersthismatch _aspc_spring_death_battle))))
    (:`CastFailed`
      (`KismetSystemLibrary.Delay` 0.2)
      (goto _label_6))))

(event `RoundStorePlayers`
  (bind _playerstart (`self.PlayerStart`))
  (`/Engine/EditorBlueprintResources/StandardMacros.DoOnce` false
    (:`Completed`
      (bind _outactors (`GameplayStatics.GetAllActorsOfClass` "/Script/Engine.PlayerStart"))
      (set `self.PlayerStart` _outactors)
      (for (_array_element _array_index) (`self.PlayersThisMatch`)
        (set `self.PlayerArray` _array_index)
        (`/Engine/EditorBlueprintResources/StandardMacros.IsValid` (`Controller.K2_GetPawn` _array_element)
          (:`Is Not Valid`
            (bind _returnvalue (`|SpawnActorFromClass` (`.PlayerCharacter_5_F87698074C265F06C9FFF08502DFEA9D` (break `/Game/SpringDeathBattle/Blueprints/Base/PlayerInfo` (`/Game/SpringDeathBattle/PC_SpringDeathBattle.PlayerInfo` _array_element))) (`self.GetTransform` (`|GetArrayItem` _playerstart (`KismetMathLibrary.RandomIntegerInRange` 0 (- (`KismetArrayLibrary.Array_Length` _playerstart) 1)))) "AdjustIfPossibleButAlwaysSpawn" "OverrideRootScale" (`|GetArrayItem` (`self.PlayersThisMatch`) (`self.PlayerArray`)) null))
            (`Controller.Possess` (`|GetArrayItem` (`self.PlayersThisMatch`) (`self.PlayerArray`)) _returnvalue)))))))

(fn `CreateCharForPlayer`
  (params (PlayerChar :type "/Game/SpringDeathBattle/Blueprints/SpringBattleBase Class Reference") (SpawnLocation :type "PlayerStart Object Reference") (PlayerController :type "/Game/SpringDeathBattle/PC_SpringDeathBattle Object Reference") (PlayerName :type Text))
  (bind _returnvalue (`|SpawnActorFromClass` PlayerChar (`self.GetTransform` SpawnLocation) "AdjustIfPossibleButDontSpawnIfColliding" "OverrideRootScale" PlayerController null))
  (`Controller.Possess` PlayerController _returnvalue)
  (`TextRenderComponent.K2_SetText` (`/Game/SpringDeathBattle/Blueprints/SpringBattleBase.TextRender` _returnvalue) PlayerName)
  (set `/Game/SpringDeathBattle/Blueprints/SpringBattleBase.Name` PlayerName _returnvalue))

(fn `PointDistribution`
  (params (GiveKill :type "/Game/SpringDeathBattle/Blueprints/SpringBattleBase Object Reference") (GiveDeath :type "/Game/SpringDeathBattle/Blueprints/SpringBattleBase Object Reference"))
  (bind _playerkills (`self.PlayerKills`))
  (bind _playerdeaths (`self.PlayerDeaths`))
  (bind _asplayer_controller (cast `PlayerController` (`Pawn.GetController` GiveKill))
    (:`then`
      (bind _aspc_spring_death_battle (cast `/Game/SpringDeathBattle/PC_SpringDeathBattle` _asplayer_controller)
        (:`then`
          (bind _returnvalue (`KismetArrayLibrary.Array_Find` (`self.PlayersThisMatch`) _aspc_spring_death_battle))
          (`KismetArrayLibrary.Array_Set` _playerkills _returnvalue (+ (`|GetArrayItem` _playerkills _returnvalue) 1)))
        (:`CastFailed`
          (`KismetSystemLibrary.PrintString` "Something Went so god darn wrong!!!! Reward" :!label _label))))
    (:`CastFailed`
      (goto _label)))
  (bind _asplayer_controller_2 (cast `PlayerController` (`Pawn.GetController` GiveDeath))
    (:`then`
      (bind _aspc_spring_death_battle_2 (cast `/Game/SpringDeathBattle/PC_SpringDeathBattle` _asplayer_controller_2)
        (:`then`
          (bind _returnvalue_2 (`KismetArrayLibrary.Array_Find` (`self.PlayersThisMatch`) _aspc_spring_death_battle_2))
          (`KismetArrayLibrary.Array_Set` _playerdeaths _returnvalue_2 (+ (`|GetArrayItem` _playerdeaths _returnvalue_2) 1)))
        (:`CastFailed`
          (`KismetSystemLibrary.PrintString` "Something Went so god darn wrong!!!! Penalty" :!label _label_2))))
    (:`CastFailed`
      (goto _label_2)))
  (`self.UpdateScoresOnClients`))

(fn `UpdateScoresOnClients`
  (for (_array_element _array_index) (`self.PlayersThisMatch`)
    (set `/Game/SpringDeathBattle/PC_SpringDeathBattle.Kills` (`|GetArrayItem` (`self.PlayerKills`) _array_index) _array_element)
    (set `/Game/SpringDeathBattle/PC_SpringDeathBattle.Deaths` (`|GetArrayItem` (`self.PlayerDeaths`) _array_index) _array_element)))

(fn `UserConstructionScript`)